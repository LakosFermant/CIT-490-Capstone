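; VertPlatform is a moving platform that shuttles back and forth between its start location and an end point given relative to it.
; BeginPlay records the start location and converts the local end offset to world space.
; Tick raises or lowers a normalized travel time scaled by TravelTime, sweeps the actor to the lerped position, and flips direction at either limit.
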(event `self.ReceiveBeginPlay`
  (bind _output_get (set `self.StartPoint` (`self.K2_GetActorLocation`)))
  (set `self.EndPointWorld` (+ (`self.EndPointLocal`) _output_get)))

(event `self.ReceiveTick`
  (params (DeltaSeconds :type "Float (single-precision)"))
  (bind _currenttraveltime (`self.currentTravelTime`))
  (bind _returnvalue (* DeltaSeconds (/ 1.0 (`self.TravelTime`))))
  (`|ExecutionSequence`
    (:`then_1`
      (if (`self.curDirection`)
        ;[1 1 1] currentTravelTime will go from 0 (0%) to 1 (100%) of the desired distance
        (set `self.currentTravelTime` (+ _returnvalue _currenttraveltime))
        (else
          (set `self.currentTravelTime` (- _currenttraveltime _returnvalue))))
      (`self.K2_SetActorLocation` (`KismetMathLibrary.VLerp` (`self.StartPoint`) (`self.EndPointWorld`) (`self.currentTravelTime`)) true)
      (if (`self.curDirection`)
        (if (>= (`self.currentTravelTime`) 1.0)
          (set `self.curDirection` false))
        (elif (<= (`self.currentTravelTime`) 0.0)
          (set `self.curDirection` true))))))

(fn `UserConstructionScript`)